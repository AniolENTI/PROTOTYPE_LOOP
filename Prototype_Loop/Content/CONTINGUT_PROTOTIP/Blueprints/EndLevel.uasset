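; EndLevel is a level exit that stays locked until the room is cleared, then sends the player on to the next level.
; Tick polls until no EnemySpawner or BP_ThirdPersonCharacter actors remain, then enables the Box collision and destroys the particle system.
; On player overlap it saves health and movement stats to MyGameInstance, then opens a random LevelArray level, or Upgrade_Room once the RoomsCompleted counter reaches three, resetting it.
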(event OnComponentBeginOverlap(Box)
  (params (OverlappedComponent :type Primitive%20Component%20Object%20Reference) (OtherActor :type Actor%20Object%20Reference) (OtherComp :type Primitive%20Component%20Object%20Reference) (OtherBodyIndex :type Integer) (bFromSweep :type Boolean) (SweepResult :type Hit%20Result%20Structure%20%28by%20ref%29))
  (bind _levelarray (Variables|Default|GetLevelArray))
  (if (== OtherActor (Game|GetPlayerCharacter 0))
    (Utilities|Casting|CastToBP_FirstPersonCharacter (Game|GetPlayerCharacter 0))
    (bind _asmy_game_instance (Utilities|Casting|CastToMyGameInstance (Game|GetGameInstance)))
    (bind _asbp_first_person_character (Utilities|Casting|CastToBP_FirstPersonCharacter (Game|GetPlayerCharacter 0)))
    (Variables|/Game/CONTINGUT_PROTOTIP/Blueprints/MyGameInstance.MyGameInstance_C|SetAirControl _asmy_game_instance (Variables|/Script/Engine.CharacterMovementComponent|GetAirControl (Variables|/Script/Engine.Character|GetCharacterMovement _asbp_first_person_character)))
    (Variables|/Game/CONTINGUT_PROTOTIP/Blueprints/MyGameInstance.MyGameInstance_C|SetCurrentHealth _asmy_game_instance (Variables|/Game/FirstPerson/Blueprints/BP_FirstPersonCharacter.BP_FirstPersonCharacter_C|GetCurrent%20Health _asbp_first_person_character))
    (Variables|/Game/CONTINGUT_PROTOTIP/Blueprints/MyGameInstance.MyGameInstance_C|SetFriction _asmy_game_instance (Variables|/Script/Engine.CharacterMovementComponent|GetGroundFriction (Variables|/Script/Engine.Character|GetCharacterMovement _asbp_first_person_character)))
    (Variables|/Game/CONTINGUT_PROTOTIP/Blueprints/MyGameInstance.MyGameInstance_C|SetJumpForce _asmy_game_instance (Variables|/Script/Engine.CharacterMovementComponent|GetJumpZVelocity (Variables|/Script/Engine.Character|GetCharacterMovement _asbp_first_person_character)))
    (Variables|/Game/CONTINGUT_PROTOTIP/Blueprints/MyGameInstance.MyGameInstance_C|SetJumps _asmy_game_instance (Variables|/Script/Engine.Character|GetJumpMaxCount _asbp_first_person_character))
    (Variables|/Game/CONTINGUT_PROTOTIP/Blueprints/MyGameInstance.MyGameInstance_C|SetMaxHealth _asmy_game_instance (Variables|/Game/FirstPerson/Blueprints/BP_FirstPersonCharacter.BP_FirstPersonCharacter_C|GetMax%20Health _asbp_first_person_character))
    (Variables|/Game/CONTINGUT_PROTOTIP/Blueprints/MyGameInstance.MyGameInstance_C|SetMaxWalkSpeed _asmy_game_instance (Variables|/Script/Engine.CharacterMovementComponent|GetMaxWalkSpeed (Variables|/Script/Engine.Character|GetCharacterMovement _asbp_first_person_character)))
    (if (not (== (Variables|/Game/CONTINGUT_PROTOTIP/Blueprints/MyGameInstance.MyGameInstance_C|GetRoomsCompleted _asmy_game_instance) 3))
      (bind _result (Math|Integer|IncrementInt (Variables|/Game/CONTINGUT_PROTOTIP/Blueprints/MyGameInstance.MyGameInstance_C|GetRoomsCompleted _asmy_game_instance))
        (:%20%20
          (Variables|/Game/CONTINGUT_PROTOTIP/Blueprints/MyGameInstance.MyGameInstance_C|SetRoomsCompleted _asmy_game_instance _result)
          (Game|OpenLevel(byObjectReference) (Utilities|Array|Get(acopy) _levelarray (Math|Random|RandomIntegerinRange 0 (- (Utilities|Array|Length _levelarray) 1))))))
      (else
        (Variables|/Game/CONTINGUT_PROTOTIP/Blueprints/MyGameInstance.MyGameInstance_C|SetRoomsCompleted _asmy_game_instance 0)
        (Game|OpenLevel(byObjectReference) "/Game/CONTINGUT_PROTOTIP/Nivells/Upgrade_Room.Upgrade_Room")))))

(event EventBeginPlay
  (Collision|SetCollisionEnabled (Variables|Default|GetBox) "NoCollision"))

(event Collision|EventActorBeginOverlap
  (params (OtherActor :type Actor%20Object%20Reference)))

(event EventTick
  (params (DeltaSeconds :type Float%20%28single-precision%29))
  (bind _particlesystem (Variables|Default|GetParticleSystem))
  (bind _outactors (Actor|GetAllActorsOfClass "/Game/CONTINGUT_PROTOTIP/Blueprints/EnemySpawner.EnemySpawner_C"))
  (if (Utilities|Array|IsEmpty _outactors)
    (bind _outactors_2 (Actor|GetAllActorsOfClass "/Game/ThirdPerson/Blueprints/BP_ThirdPersonCharacter.BP_ThirdPersonCharacter_C"))
    (if (Utilities|Array|IsEmpty _outactors_2)
      (Collision|SetCollisionEnabled (Variables|Default|GetBox) "QueryAndPhysics")
      (if (Utilities|IsValid _particlesystem)
        (Components|DestroyComponent _particlesystem)
        (Utilities|Platform|CollectGarbage)))))

(fn ConstructionScript)