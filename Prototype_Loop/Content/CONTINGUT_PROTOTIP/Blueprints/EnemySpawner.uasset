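; EnemySpawner is a spawner actor that creates BP_ThirdPersonCharacter instances at its own transform when play begins.
; SpawnEnemy spawns one immediately, then re-calls itself after a short random delay, decrementing EnemyAmount each time.
; The loop stops once EnemyAmount is no longer above one, so the variable sets the total spawn count, with a minimum of one.
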(event Custom|SpawnEnemy
  (Game|SpawnActorfromClass "/Game/ThirdPerson/Blueprints/BP_ThirdPersonCharacter.BP_ThirdPersonCharacter_C" (Transformation|GetActorTransform) "Undefined" "MultiplyWithRoot" 0 0)
  (if (> (Variables|Default|GetEnemyAmount) 1)
    (Utilities|FlowControl|Delay (Math|Random|RandomFloatinRange 1.0 2.5))
    (Math|Integer|DecrementInt (Variables|Default|GetEnemyAmount)
      (:%20%20
        (CallFunction|SpawnEnemy)))))

(event EventBeginPlay
  (CallFunction|SpawnEnemy))

(fn ConstructionScript)